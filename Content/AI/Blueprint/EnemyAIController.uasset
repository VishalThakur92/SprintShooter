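; AI controller for enemies that starts their behavior tree and seeds its combat range settings.
; On possess, a sequence runs BT_Enemy, then copies the controller's shooting and melee distance variables into Blackboard keys.
; It then finds the level's FlankManager actor and caches a reference, which this graph does not use further.
; Debug prints for both distance keys are left unconnected.
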(event `self.ReceivePossess`
  (params (PossessedPawn :type "Pawn Object Reference"))
  (`|ExecutionSequence`
    (:`then_0`
      ;[0.07561 1 0] Run Behaviour Tree
      (`self.RunBehaviorTree` "/Game/AI/Blueprint/BehaviourTree/BT_Enemy.BT_Enemy"))
    (:`then_1`
      ;[1 0.7026 0] Initialize Blackboard key value for Shooting Distance
      (`BlackboardComponent.SetValueAsFloat` (`AIBlueprintHelperLibrary.GetBlackboard` null) "ShootDistance" (`self.ShootingDistance`)))
    (:`then_2`
      ;[1 0.7026 0] Initialize Blackboard key value for Meele Distance
      (`BlackboardComponent.SetValueAsFloat` (`AIBlueprintHelperLibrary.GetBlackboard` null) "MeeleDistance" (`self.MeeleDistance`)))
    (:`then_3`
      ;[0 0 0] Find and Save FlankManager Ref
      (bind _returnvalue (`GameplayStatics.GetActorOfClass` "/Game/AI/Blueprint/Managers/FlankManager.FlankManager_C"))
      (set `self.FlankManager` _returnvalue))))

(fn `UserConstructionScript`)