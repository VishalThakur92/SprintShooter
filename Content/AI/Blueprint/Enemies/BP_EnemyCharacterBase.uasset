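; Base enemy character Blueprint that detects the player through Pawn Sensing and reports it to its AI Blackboard.
; On seeing the first-person character, it stores the distance to the player and sets the HasSeenPlayer key to true.
; A retriggerable delay clears the key shortly after sightings stop.
; Tick does no work, and a distance debug print is left disconnected.
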(event `self.PawnSensing.OnSeePawn`
  (params (Pawn :type "Pawn Object Reference"))
  (bind _returnvalue (`AIBlueprintHelperLibrary.GetBlackboard` (`AIBlueprintHelperLibrary.GetAIController` self)))
  ;[0 0 0] On Player Detected Behaviour
  (cast `/Game/FirstPerson/Blueprints/BP_FirstPersonCharacter` Pawn)
  (`|ExecutionSequence`
    (:`then_0`
      ;;[0 0 0] Get distance from player and save it
      (bind _distance (`self.GetDistanceFromPlayer`))
      (set `self.DistanceFromPlayer` _distance))
    (:`then_1`
      ;;[0 0 0] Update Blackboard's HasSeenPlayer key
      (`BlackboardComponent.SetValueAsBool` _returnvalue "HasSeenPlayer" true))
    (:`then_2`
      (`KismetSystemLibrary.RetriggerableDelay` 2.0)
      (`BlackboardComponent.SetValueAsBool` _returnvalue "HasSeenPlayer" false))))

(event `self.ReceiveTick`
  (params (DeltaSeconds :type "Float (single-precision)"))
  ;[0 0 0] Event Tick Stuff
  (`|ExecutionSequence`))

(fn `GetDistanceFromPlayer`
  (returns (Distance :type "Float (double-precision)"))
  (return (`KismetMathLibrary.Vector_Distance` (`self.K2_GetActorLocation`) (`self.K2_GetActorLocation` (`GameplayStatics.GetPlayerCharacter` 0)))))

(fn `UserConstructionScript`)