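; Base walking enemy character Blueprint that handles flank positioning and jumping for its AI.
; It requests the closest flank position from the FlankManager on its EnemyWalkingAIController and tracks whether it holds a valid one.
; When the player moves, it releases that position for other enemies and stops reacting to further moves until it requests another.
; JumptoDestination launches the character along a suggested projectile arc with a height offset.
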(event `/Game/AI/Interface/PlayerMovementListener.OnPlayerMoved`
  ;[0 0 0] Player Has moved, so will need to get a new flank position
  (if (`self.ListenToPlayerMovedEvent`)
    (`self.RequestReleaseFlankPosition`)))

(event `/Game/AI/Interface/Jumpable.JumpToDestination`
  (params (Destination :type "Vector Structure"))
  (bind _outlaunchvelocity (`GameplayStatics.SuggestProjectileVelocity_CustomArc` (`self.K2_GetActorLocation`) (`KismetMathLibrary.MakeVector` Destination_X Destination_Y (+ Destination_Z (`self.JumpOffset`)))))
  (`self.LaunchCharacter` _outlaunchvelocity true true))

(fn `RequestFlankPosition`
  (params (MyPosition :type "Vector Structure"))
  ;[0 0 0] Request a flank position from FlankManager
  (bind _asenemy_walking_aicontroller (cast `/Game/AI/Blueprint/Enemies/Walking/EnemyWalkingAIController` (`AIBlueprintHelperLibrary.GetAIController` self))
    (:`then`
      (bind _flankposition (`/Game/AI/Blueprint/Managers/FlankManager.GetClosestFlankPosition` (`/Game/AI/Blueprint/Enemies/Walking/EnemyWalkingAIController.FlankManager` _asenemy_walking_aicontroller) MyPosition))
      (set `self.FlankPosition` _flankposition)
      (set `self.HasValidFlankPosition` true)
      (set `self.ListenToPlayerMovedEvent` true)
      (return))
    (:`CastFailed`
      (`KismetSystemLibrary.PrintString` "Cast Failed To EnemyAIController"))))

(fn `RequestReleaseFlankPosition`
  ;[0 0 0] Release my Flank position for other enemies to use
  (bind _asenemy_walking_aicontroller (cast `/Game/AI/Blueprint/Enemies/Walking/EnemyWalkingAIController` (`AIBlueprintHelperLibrary.GetAIController` self)))
  (`/Game/AI/Blueprint/Managers/FlankManager.ReleaseFlankPosition` (`/Game/AI/Blueprint/Enemies/Walking/EnemyWalkingAIController.FlankManager` _asenemy_walking_aicontroller) (`self.FlankPosition`))
  (set `self.ListenToPlayerMovedEvent` false)
  (set `self.HasValidFlankPosition` false))

(fn `UserConstructionScript`)