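; Sniper enemy character Blueprint that can leap to a destination and provides a vantage point lookup.
; JumptoDestination launches the character along a suggested custom-arc projectile velocity, with a height offset added to the destination.
; GetNextVantagePoint compares a random array entry to the current target and recurses on a match to avoid repeats.
; Its non-matching branch reassigns the current target to itself, so the random pick is never stored.
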(event `/Game/AI/Interface/Jumpable.JumpToDestination`
  (params (Destination :type "Vector Structure"))
  (bind _outlaunchvelocity (`GameplayStatics.SuggestProjectileVelocity_CustomArc` (`self.K2_GetActorLocation`) (`KismetMathLibrary.MakeVector` Destination_X Destination_Y (+ Destination_Z (`self.JumpOffset`)))))
  (`self.LaunchCharacter` _outlaunchvelocity true true))

(fn `GetNextVantagePoint`
  (returns (VantagePoint :type "Vector Structure"))
  (bind _targetvantagepoint (`self.TargetVantagePoint`))
  ;[0 0 0] Get a random Vantage Point from the Array
  ;;[0 0 0] Donot get same vantage point
  (if (== (`KismetArrayLibrary.Array_Random` (`self.VantagePoints`)) _targetvantagepoint)
    (bind _vantagepoint (`self.GetNextVantagePoint`))
    (bind _output_get (set `self.TargetVantagePoint` _vantagepoint))
    (return _output_get)
    (else
      (bind _output_get_2 (set `self.TargetVantagePoint` _targetvantagepoint))
      (return _output_get_2))))

(fn `UserConstructionScript`)