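; Flank manager that hands out attack positions in a ring around player 0 for enemies to use.
; On BeginPlay and every Tick it rebuilds evenly angled points at the flank radius from the player's location, then draws debug boxes marking assigned or free.
; GetAttackPosition reserves the first unassigned point and ReleaseFlankPosition frees it.
; Reservations match by exact vector value, so they stop matching rebuilt points when the player moves.
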(event `self.ReceiveBeginPlay`
  (`self.CalculateFlankPositions` :!label _label)
  (`self.DebugFlankPositions`))

(event `self.ReceiveTick`
  (params (DeltaSeconds :type "Float (single-precision)"))
  (goto _label))

(fn `CalculateFlankPositions`
  (locals (XOffset :type "Float (double-precision)") (YOffset :type "Float (double-precision)"))
  (bind _flankradius (`self.FlankRadius`))
  (bind (_returnvalue_x _returnvalue_y _returnvalue_z) (`KismetMathLibrary.BreakVector` (`self.K2_GetActorLocation` (`GameplayStatics.GetPlayerCharacter` 0))))
  (`KismetArrayLibrary.Array_Clear` (`self.AvailableFlankPositions`))
  (for _index (range (+ (`self.MaxFlankPositions`) 1))
    (bind _returnvalue (`KismetMathLibrary.DegreesToRadians` (* (/ (`KismetMathLibrary.Conv_IntToDouble` _index) (`KismetMathLibrary.Conv_IntToDouble` (`self.MaxFlankPositions`))) 360.0)))
    ;[0 0 0] Divide the current index by the total number of positions, multiply by 360, and convert to radians.
    (set `local.XOffset` (* (`KismetMathLibrary.Cos` _returnvalue) _flankradius))
    (set `local.YOffset` (* _flankradius (`KismetMathLibrary.Sin` _returnvalue)))
    ;[0 0 0] Create the position vector using X, Y, and the player's Z location, and then add it to the availablePositions Array
    (`KismetArrayLibrary.Array_AddUnique` (`self.AvailableFlankPositions`) (`KismetMathLibrary.MakeVector` (+ _returnvalue_x (`local.XOffset`)) (+ _returnvalue_y (`local.YOffset`)) _returnvalue_z))))

(fn `DebugFlankPositions`
  (for _array_element (`self.AvailableFlankPositions`)
    (if (`KismetArrayLibrary.Array_Contains` (`self.AssignedFlankPositions`) _array_element)
      (`KismetSystemLibrary.DrawDebugBox` _array_element (5.0 5.0 5.0) (struct :`R` 1.0 :`B` 0.05385 :`A` 1.0) (struct) 0.1 20.0)
      (else
        (`KismetSystemLibrary.DrawDebugBox` _array_element (5.0 5.0 5.0) (struct :`G` 1.0 :`B` 0.063156 :`A` 1.0) (struct) 0.1 20.0)))))

(fn `GetAttackPosition`
  (returns (FlankPosition :type "Vector Structure"))
  (for _array_element (`self.AvailableFlankPositions`)
    (if (not (`KismetArrayLibrary.Array_Contains` (`self.AssignedFlankPositions`) _array_element))
      (`KismetArrayLibrary.Array_AddUnique` (`self.AssignedFlankPositions`) _array_element)
      (return _array_element))))

(fn `ReleaseFlankPosition`
  (params (Position :type "Vector Structure"))
  ;[0 0 0] Once an enemy dies or leaves the flank position, remove it from assigned position for other enemies to use
  (if (`KismetArrayLibrary.Array_Contains` (`self.AssignedFlankPositions`) Position)
    (`KismetArrayLibrary.Array_RemoveItem` (`self.AssignedFlankPositions`) Position)))

(fn `UserConstructionScript`)