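; Behavior tree task that makes an AI enemy chase the player.
; On execute it casts the controlled pawn to BP_AI and resets the attack pose on its ABP_Enemy animation instance.
; It then runs AI MoveTo toward player character 0 with a wide acceptance radius, finishing the task as succeeded or failed to match the move result.
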(event `self.ReceiveExecuteAI`
  (params (OwnerController :type "AIController Object Reference") (ControlledPawn :type "Pawn Object Reference"))
  ;[0 0 0] Move to Player's location
  (bind _output_get (set `self.Controlled Pawn` ControlledPawn))
  (bind _asbp_ai (cast `/Game/AI/Blueprint/BP_AI` _output_get))
  (bind _asabp_enemy (cast `/Game/AI/Blueprint/ABP_Enemy` (`SkeletalMeshComponent.GetAnimInstance` (`Character.Mesh` _asbp_ai))))
  (`/Game/AI/Blueprint/ABP_Enemy.ResetAttackPose` _asabp_enemy)
  (`|AIMoveTo` (`self.Controlled Pawn`) (0.0 0.0 0.0) (`GameplayStatics.GetPlayerCharacter` 0) 700.0
    (:`OnSuccess`
      (`self.FinishExecute` true))
    (:`OnFail`
      (`self.FinishExecute` false))))