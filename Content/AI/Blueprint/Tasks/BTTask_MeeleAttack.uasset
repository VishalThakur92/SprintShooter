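; Behavior tree task that makes an enemy AI pawn perform a melee attack.
; It casts the pawn to BP_AI and its mesh's anim instance to ABP_Enemy, then calls PlayMeeleAnimation.
; It also snaps the pawn's rotation to face player 0 once per execution and finishes successfully right away, without waiting for the animation.
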(event `self.ReceiveExecuteAI`
  (params (OwnerController :type "AIController Object Reference") (ControlledPawn :type "Pawn Object Reference"))
  (set `self.Controlled Pawn` ControlledPawn)
  (`|ExecutionSequence`
    (:`then_0`
      ;[0 0 0] Meele Behaviour
      ;;[0 0 0] Play Meele animation
      (bind _asbp_ai (cast `/Game/AI/Blueprint/BP_AI` (`self.Controlled Pawn`)))
      (bind _asabp_enemy (cast `/Game/AI/Blueprint/ABP_Enemy` (`SkeletalMeshComponent.GetAnimInstance` (`Character.Mesh` _asbp_ai))))
      (`/Game/AI/Blueprint/ABP_Enemy.PlayMeeleAnimation` _asabp_enemy))
    (:`then_1`
      ;;[0 0 0] Always Look at player
      (`Actor.K2_SetActorRotation` (`self.Controlled Pawn`) (`KismetMathLibrary.MakeRotFromX` (`KismetMathLibrary.GetDirectionUnitVector` (`Actor.K2_GetActorLocation` (`self.Controlled Pawn`)) (`Actor.K2_GetActorLocation` (`GameplayStatics.GetPlayerPawn` 0)))) false))
    (:`then_2`
      (`self.FinishExecute` true))))