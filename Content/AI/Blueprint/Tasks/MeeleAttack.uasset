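; MeeleAttack is an AI Behavior Tree task that makes a walking enemy perform a melee attack facing the player.
; It casts the pawn to BP_EnemyCharacterWalking and calls PlayMeeleAnimation on its ABP_EnemyWalking anim instance.
; It then snaps the pawn's rotation toward player character 0, flattened to the horizontal plane.
; The task finishes successfully at once, without waiting for the animation or depending on the casts.
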(event `self.ReceiveExecuteAI`
  (params (OwnerController :type "AIController Object Reference") (ControlledPawn :type "Pawn Object Reference"))
  (bind (_returnvalue_x _returnvalue_y) (`KismetMathLibrary.BreakVector` (`KismetMathLibrary.GetDirectionUnitVector` (`Actor.K2_GetActorLocation` (`self.Controlled Pawn`)) (`Actor.K2_GetActorLocation` (`GameplayStatics.GetPlayerCharacter` 0)))))
  (set `self.Controlled Pawn` ControlledPawn)
  (`|ExecutionSequence`
    (:`then_0`
      ;[0 0 0] Meele Behaviour
      ;;[0 0 0] Play Meele animation
      (bind _asbp_enemy_character_walking (cast `/Game/AI/Blueprint/Enemies/Walking/BP_EnemyCharacterWalking` (`self.Controlled Pawn`)))
      (bind _asabp_enemy_walking (cast `/Game/AI/Blueprint/Enemies/Walking/ABP_EnemyWalking` (`SkeletalMeshComponent.GetAnimInstance` (`Character.Mesh` _asbp_enemy_character_walking))))
      (`/Game/AI/Blueprint/Enemies/Walking/ABP_EnemyWalking.PlayMeeleAnimation` _asabp_enemy_walking))
    (:`then_1`
      ;;[0 0 0] Always Look at player
      (`Actor.K2_SetActorRotation` (`self.Controlled Pawn`) (`KismetMathLibrary.MakeRotFromX` (`KismetMathLibrary.MakeVector` _returnvalue_x _returnvalue_y)) false))
    (:`then_2`
      (`self.FinishExecute` true))))