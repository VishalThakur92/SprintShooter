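; Behavior tree task that sends a walking enemy running toward the player character.
; It casts the controlled pawn and its mesh's anim instance to the walking enemy types, then resets the attack pose.
; AI MoveTo targets player 0 with a wide acceptance radius and finishes the task with the move's success or failure.
; A failed cast stops execution without finishing the task.
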(event `self.ReceiveExecuteAI`
  (params (OwnerController :type "AIController Object Reference") (ControlledPawn :type "Pawn Object Reference"))
  ;[0 0 0] Run to Player
  (bind _output_get (set `self.Controlled Pawn` ControlledPawn))
  (bind _asbp_enemy_character_walking (cast `/Game/AI/Blueprint/Enemies/Walking/BP_EnemyCharacterWalking` _output_get))
  (bind _asabp_enemy_walking (cast `/Game/AI/Blueprint/Enemies/Walking/ABP_EnemyWalking` (`SkeletalMeshComponent.GetAnimInstance` (`Character.Mesh` _asbp_enemy_character_walking))))
  (`/Game/AI/Blueprint/Enemies/Walking/ABP_EnemyWalking.ResetAttackPose` _asabp_enemy_walking)
  (`|AIMoveTo` (`self.Controlled Pawn`) (0.0 0.0 0.0) (`GameplayStatics.GetPlayerCharacter` 0) 700.0
    (:`OnSuccess`
      (`self.FinishExecute` true))
    (:`OnFail`
      (`self.FinishExecute` false))))