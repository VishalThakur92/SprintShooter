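; BP_AI is an enemy AI pawn that spots the player through PawnSensing.
; Seeing the first-person character sets the HasSeenPlayer blackboard key true, and a one-second retriggerable delay clears it once sightings stop.
; A helper computes the truncated distance to the player, but its calls and debug print are unconnected, so they never run.
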(event `self.ReceiveTick`
  (params (DeltaSeconds :type "Float (single-precision)")))

(event `self.PawnSensing.OnSeePawn`
  (params (Pawn :type "Pawn Object Reference"))
  (bind _returnvalue (`AIBlueprintHelperLibrary.GetBlackboard` (`AIBlueprintHelperLibrary.GetAIController` self)))
  ;[0 0 0] Enemy has seen the Player, update the blackboard  key
  (cast `/Game/FirstPerson/Blueprints/BP_FirstPersonCharacter` Pawn)
  (`|ExecutionSequence`
    (:`then_0`
      (`BlackboardComponent.SetValueAsBool` _returnvalue "HasSeenPlayer" true))
    (:`then_1`
      (`KismetSystemLibrary.RetriggerableDelay` 1.0)
      (`BlackboardComponent.SetValueAsBool` _returnvalue "HasSeenPlayer" false))))

(fn `CalculateDistanceFromPlayer`
  (returns (Distance :type Integer))
  ;[0 0 0] Calculate AIPawn's distance from the player pawn
  (return (`KismetMathLibrary.FTrunc` (`KismetMathLibrary.Vector_Distance` (`self.K2_GetActorLocation`) (`self.K2_GetActorLocation` (`GameplayStatics.GetPlayerCharacter` 0))))))

(fn `UserConstructionScript`)