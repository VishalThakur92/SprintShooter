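; CanShoot is an AI behavior tree decorator that passes when the pawn's distance falls within shooting range but outside melee range.
; Its condition check casts the controlled pawn to BP_AI and reads its Distance variable.
; That value must be greater than the blackboard melee distance and no greater than the blackboard shooting distance, both read through key selectors.
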(fn `PerformConditionCheckAI`
  (params (OwnerController :type "AIController Object Reference") (ControlledPawn :type "Pawn Object Reference"))
  (returns (ReturnValue :type Boolean))
  ;[0 0 0] If Distance greater than meele but less than shooting distance
  (bind _asbp_ai (cast `/Game/AI/Blueprint/BP_AI` ControlledPawn))
  (bind _output_get (set `self.Distance` (`/Game/AI/Blueprint/BP_AI.Distance` _asbp_ai)))
  (return (and (> _output_get (`BTFunctionLibrary.GetBlackboardValueAsFloat` (`self.MeeleDistanceKey`))) (<= (`self.Distance`) (`BTFunctionLibrary.GetBlackboardValueAsFloat` (`self.ShootingDistanceKey`))))))